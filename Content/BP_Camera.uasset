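; BP_Camera is a camera actor that sweeps back and forth and locks onto a pawn it detects.
; DetectionCone overlaps with "Pawn"-tagged actors and a per-tick visibility trace from CameraBody to the first pawn found at BeginPlay together set IsLockedOn.
; When locked, CameraBase yaws and CameraBody yaws and tilts to face that pawn.
; Otherwise, the actor eases through a sine-driven yaw sweep around its starting rotation.
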(event OnComponentBeginOverlap(DetectionCone)
  (params (OverlappedComponent :type Primitive%20Component%20Object%20Reference) (OtherActor :type Actor%20Object%20Reference) (OtherComp :type Primitive%20Component%20Object%20Reference) (OtherBodyIndex :type Integer) (bFromSweep :type Boolean) (SweepResult :type Hit%20Result%20Structure%20%28by%20ref%29))
  (if (Actor|ActorHasTag OtherActor "Pawn")
    (Variables|Default|SetPawnCollision true)))

(event OnComponentEndOverlap(DetectionCone)
  (params (OverlappedComponent :type Primitive%20Component%20Object%20Reference) (OtherActor :type Actor%20Object%20Reference) (OtherComp :type Primitive%20Component%20Object%20Reference) (OtherBodyIndex :type Integer))
  (if (Actor|ActorHasTag OtherActor "Pawn")
    (Variables|Default|SetPawnCollision false)))

(event EventBeginPlay
  (Variables|Default|SetRotOffset (.Yaw (Math|Rotator|BreakRotator (Transformation|GetActorRotation))))
  (bind _outactors (Actor|GetAllActorsOfClass "/Script/Engine.Pawn"))
  (if (Utilities|Array|IsValidIndex _outactors)
    (Variables|Default|SetTarget%20Pawn (Utilities|Array|Get(acopy) _outactors))))

(event Collision|EventActorBeginOverlap
  (params (OtherActor :type Actor%20Object%20Reference)))

(event EventTick
  (params (DeltaSeconds :type Float%20%28single-precision%29))
  (bind _returnvalue (Transformation|GetActorLocation))
  (bind _returnvalue_2 (Transformation|GetActorRotation))
  (bind _target_pawn (Variables|Default|GetTarget%20Pawn))
  (bind (_roll _pitch) (Math|Rotator|BreakRotator _returnvalue_2))
  (bind _returnvalue_3 (Transformation|GetActorLocation _target_pawn))
  (bind _returnvalue_4 (Math|Rotator|FindLookatRotation _returnvalue_3 _returnvalue))
  (bind (_roll_2 _pitch_2 _yaw) (Math|Rotator|BreakRotator _returnvalue_4))
  (bind _returnvalue_5 (+ _yaw 9e+01))
  (bind (_outhit _returnvalue_6) (Collision|LineTraceByChannel (Transformation|GetWorldLocation (Variables|Default|GetCameraBody)) (Transformation|GetWorldLocation (Variables|/Script/Engine.Actor|GetRootComponent (Variables|Default|GetTarget%20Pawn))) "TraceTypeQuery1" false 0 "None"))
  (if _returnvalue_6
    (bind _output_get (Variables|Default|SetPawnRaycast (Actor|ActorHasTag (.HitActor (Collision|BreakHitResult _outhit)) "Pawn"))))
  (bind _output_get_2 (Variables|Default|SetIsLockedOn (and _output_get (Variables|Default|GetPawnCollision))))
  (if _output_get_2
    (Transformation|SetWorldRotation (Variables|Default|GetCameraBody) (Math|Rotator|MakeRotator _pitch_2 0.0 _returnvalue_5) false false)
    (Transformation|SetWorldRotation (Variables|Default|GetCameraBase) (Math|Rotator|MakeRotator 0.0 0.0 _returnvalue_5) false false)
    (else
      (Transformation|SetActorRotation (Math|Interpolation|RInterpTo (Transformation|GetActorRotation) (Math|Rotator|MakeRotator _roll _pitch (+ (Math|Float|Lerp 0.0 45.0 (Math|Trig|Sin(Degrees) (* (Utilities|Time|GetGameTimeinSeconds) 15.0))) (Variables|Default|GetRotOffset))) DeltaSeconds 0.5)))))

(fn ConstructionScript)