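; BP_Detector is an actor that turns to face a pawn and reports what lies in its line of sight.
; On BeginPlay it stores the first Pawn found in the level as its target.
; Each Tick it rotates toward that pawn, line-traces on the Visibility channel along the Sphere component's forward vector, draws the trace and prints the hit actor's name.
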(event EventBeginPlay
  (bind _outactors (Actor|GetAllActorsOfClass "/Script/Engine.Pawn"))
  (if (Utilities|Array|IsValidIndex _outactors)
    (Variables|Default|SetTargetPawn (Utilities|Array|Get(acopy) _outactors))))

(event Collision|EventActorBeginOverlap
  (params (OtherActor :type Actor%20Object%20Reference)))

(event EventTick
  (params (DeltaSeconds :type Float%20%28single-precision%29))
  (bind _sphere (Variables|Default|GetSphere))
  (bind _returnvalue (Transformation|GetWorldLocation _sphere))
  (bind _targetpawn (Variables|Default|GetTargetPawn)
    (:then
      (Transformation|SetActorRotation (Math|Rotator|FindLookatRotation (Transformation|GetActorLocation) (Transformation|GetActorLocation _targetpawn)))
      (bind _outhit (Collision|LineTraceByChannel _returnvalue (+ _returnvalue (* (Math|Vector|GetForwardVector (Transformation|GetWorldRotation _sphere)) 2e+03)) "TraceTypeQuery1" false 0 "ForOneFrame"))
      (Development|PrintString (Utilities|GetDisplayName (.HitActor (Collision|BreakHitResult _outhit)))))
    (:else)))

(fn ConstructionScript)